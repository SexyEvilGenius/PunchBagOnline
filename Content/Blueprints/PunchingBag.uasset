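; PunchingBag is an actor that exercises a MotionInterpolator component, with debug visuals for snapshots and ownership.
; The interpolator activates five seconds after BeginPlay, and TakeAuthority passes release delay and blend-out timing to its movement authority takeover.
; Each added snapshot draws a brief, scale-sized debug sphere at its location.
; A text render shows the current owner's object name, refreshed every tick.
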(event `self.ReceiveBeginPlay`
  (`KismetSystemLibrary.Delay` 5.0)
  (`ActorComponent.Activate` (`self.MotionInterpolator`) true))

(event `self.ReceiveTick`
  (params (DeltaSeconds :type "Float (single-precision)"))
  (`TextRenderComponent.K2_SetText` (`self.TextRender`) (`KismetTextLibrary.Conv_StringToText` (`KismetSystemLibrary.GetObjectName` (`self.GetOwner`)))))

(event `TakeAuthority`
  (params (InReleaseDelay :type "Float (double-precision)") (BlendOutDuration :type "Float (double-precision)"))
  (`MotionInterpolatorComponent.OvertakeMovementAuthority` (`self.MotionInterpolator`) InReleaseDelay BlendOutDuration))

(event `self.MotionInterpolator.OnSnapshotAdded`
  (params (Snapshot :type "MotionSnapshot Structure (by ref)"))
  (`KismetSystemLibrary.DrawDebugSphere` Snapshot_Location (* 60.0 (`KismetMathLibrary.GetMaxElement` (`self.GetActorScale3D`))) 12 (struct :`R` 1.0 :`B` 0.078031 :`A` 1.0) 0.5 0.1))

(fn `UserConstructionScript`)