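; PBOPawn is a pawn that shows its player's name on a TextRender component and raises its HMD component once play has started.
; Five seconds after BeginPlay, the authority sets GameStarted, which has an empty OnRep handler.
; While the flag is set and PlayerState is valid, Tick refreshes the name text and teleports HMD one unit along local Z every frame, independent of delta time.
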(event `self.ReceiveBeginPlay`
  (`KismetSystemLibrary.Delay` 5.0)
  (`/Engine/EditorBlueprintResources/ActorMacros.Switch Has Authority`
    (:`Authority`
      (set `self.GameStarted` true))))

(event `self.ReceiveTick`
  (params (DeltaSeconds :type "Float (single-precision)"))
  (if (`self.GameStarted`)
    (bind _playerstate (`self.PlayerState`)
      (:`then`
        (`TextRenderComponent.K2_SetText` (`self.TextRender`) (`KismetTextLibrary.Conv_StringToText` (`PlayerState.GetPlayerName` _playerstate)))
        (`SceneComponent.K2_AddLocalOffset` (`self.HMD`) (0.0 0.0 1.0) false true))
      (:`else`))))

(fn `OnRep_GameStarted`)

(fn `UserConstructionScript`)